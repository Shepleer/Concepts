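; Animation modifier that automatically places left and right foot sync markers on animation sequences.
; On apply, it optionally clears existing markers, adds notify tracks, then samples root motion and component-space foot and trajectory reference bone positions at a fixed step.
; A marker lands where a foot's offset from the reference bone, dotted with root motion translation, flips from positive to negative.
; Revert removes both tracks.
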(event EventOnApply
  (params (AnimationSequence :type Anim%20Sequence%20Object%20Reference))
  (if (Variables|Default|GetRemovePreExistingSyncMarkers)
    (Class|AnimationBlueprintLibrary|RemoveAllAnimationSyncMarkers AnimationSequence))
  (Class|AnimationBlueprintLibrary|AddAnimationNotifyTrack AnimationSequence (Variables|Default|GetLeftFootNotifyTrackName) "(R=1.000000,G=1.000000,B=1.000000,A=1.000000)")
  (if (!= (Variables|Default|GetLeftFootNotifyTrackName) (Variables|Default|GetRightFootNotifyTrackName))
    (Class|AnimationBlueprintLibrary|AddAnimationNotifyTrack AnimationSequence (Variables|Default|GetRightFootNotifyTrackName) "(R=1.000000,G=1.000000,B=1.000000,A=1.000000)"))
  (for _index (range 0 (Math|Float|Truncate (/ (Class|AnimationBlueprintLibrary|GetSequenceLength AnimationSequence) (Variables|Default|GetSampleStep))))
    (CallFunction|DetectMarkerforTime (* _index (Variables|Default|GetSampleStep)) AnimationSequence)))

(event EventOnRevert
  (params (AnimationSequence :type Anim%20Sequence%20Object%20Reference))
  (Class|AnimationBlueprintLibrary|RemoveAnimationNotifyTrack AnimationSequence (Variables|Default|GetLeftFootNotifyTrackName))
  (Class|AnimationBlueprintLibrary|RemoveAnimationNotifyTrack AnimationSequence (Variables|Default|GetRightFootNotifyTrackName)))

(fn ShouldPlaceMarkerforFoot
  (params (RootMotionTranslation :type Vector) (FootPos :type Vector) (TrajectoryPos :type Vector) (LastDotProduct :type Float%20%28double-precision%29))
  (bind _returnvalue (- FootPos TrajectoryPos))
  (bind _returnvalue_2 (Math|Vector|DotProduct RootMotionTranslation _returnvalue))
  ;[1 1 1] Test if the foot was ahead of the trajectory reference bone (in direction of root motion) but is now behind.
  (return _returnvalue_2 (and (< _returnvalue_2 0.0) (> LastDotProduct 0.0))))

(fn GetBoneComponentSpaceTransform
  (params (AnimSequence :type Anim%20Sequence%20Base%20Object%20Reference) (BoneName :type Name) (Time :type Float%20%28double-precision%29))
  (for _array_element (Class|AnimationBlueprintLibrary|GetBonePosesforTime AnimSequence (Class|AnimationBlueprintLibrary|FindBonePathtoRoot AnimSequence BoneName) Time false 0)
    (LocalVariables|SetLocalAccumulatedTransform (Math|Transform|ComposeTransforms (LocalVariables|GetLocalAccumulatedTransform) _array_element)))
  (return (LocalVariables|GetLocalAccumulatedTransform)))

(fn DetectMarkerforTime
  (params (Time :type Float%20%28double-precision%29) (AnimSequence :type Anim%20Sequence%20Base%20Object%20Reference))
  (LocalVariables|SetLocalTime Time)
  (bind _asanim_sequence (Utilities|Casting|CastToAnimSequence AnimSequence))
  (LocalVariables|SetLocalAnimSequence _asanim_sequence)
  (Utilities|FlowControl|Sequence
    (:then_0
      ;[1 1 1] Get root motion translation
      (LocalVariables|SetLocalRootMotionTranslation (CallFunction|ExtractRootMotion (LocalVariables|GetLocalAnimSequence) (LocalVariables|GetLocalTime) (+ (LocalVariables|GetLocalTime) (Variables|Default|GetSampleStep)))))
    (:then_1
      ;[1 1 1] Get trajectory reference bone position
      (LocalVariables|SetLocalTrajRefBonePos (.location (CallFunction|GetBoneComponentSpaceTransform (LocalVariables|GetLocalAnimSequence) (Variables|Default|GetTrajectoryReferenceBoneName) (LocalVariables|GetLocalTime)))))
    (:then_2
      ;[1 1 1] Get left foot bone position
      (LocalVariables|SetLocalLeftBonePos (.location (CallFunction|GetBoneComponentSpaceTransform (LocalVariables|GetLocalAnimSequence) (Variables|Default|GetLeftFootBoneName) (LocalVariables|GetLocalTime)))))
    (:then_3
      ;[1 1 1] Right right foot bone position
      (LocalVariables|SetLocalRightBonePos (.location (CallFunction|GetBoneComponentSpaceTransform (LocalVariables|GetLocalAnimSequence) (Variables|Default|GetRightFootBoneName) (LocalVariables|GetLocalTime)))))
    (:then_4
      ;[1 1 1] Place marker for left foot if desired
      (bind (_currentdotproduct _shouldplacemarker) (CallFunction|ShouldPlaceMarkerforFoot (LocalVariables|GetLocalRootMotionTranslation) (LocalVariables|GetLocalLeftBonePos) (LocalVariables|GetLocalTrajRefBonePos) (Variables|Default|GetLastLeftFootDotProduct)))
      (Variables|Default|SetLastLeftFootDotProduct _currentdotproduct)
      (if _shouldplacemarker
        (Class|AnimationBlueprintLibrary|AddAnimationSyncMarker (LocalVariables|GetLocalAnimSequence) (Variables|Default|GetLeftFootMarkerName) (LocalVariables|GetLocalTime) (Variables|Default|GetLeftFootNotifyTrackName))))
    (:then_5
      ;[1 1 1] Place marker for right foot if desired
      (bind (_currentdotproduct_2 _shouldplacemarker_2) (CallFunction|ShouldPlaceMarkerforFoot (LocalVariables|GetLocalRootMotionTranslation) (LocalVariables|GetLocalRightBonePos) (LocalVariables|GetLocalTrajRefBonePos) (Variables|Default|GetLastRightFootDotProduct)))
      (Variables|Default|SetLastRightFootDotProduct _currentdotproduct_2)
      (if _shouldplacemarker_2
        (Class|AnimationBlueprintLibrary|AddAnimationSyncMarker (LocalVariables|GetLocalAnimSequence) (Variables|Default|GetRightFootMarkerName) (LocalVariables|GetLocalTime) (Variables|Default|GetRightFootNotifyTrackName))))))

(fn ExtractRootMotion
  (params (Animation :type Anim%20Sequence%20Object%20Reference) (StartTime :type Float%20%28double-precision%29) (EndTime :type Float%20%28double-precision%29))
  (bind _rootbonename (Variables|Default|GetRootBoneName))
  (return (- (.location (Class|AnimationBlueprintLibrary|GetBonePoseforTime Animation _rootbonename (Math|Float|Clamp(Float) EndTime 0.0 (Animation|GetPlayLength Animation)) true)) (.location (Class|AnimationBlueprintLibrary|GetBonePoseforTime Animation _rootbonename StartTime true)))))